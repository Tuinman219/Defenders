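; Commander_BP is a player character with mouse look, jumping and a hold-to-attack melee combo using Serath montages.
; Left mouse sets a held flag that Tick polls, starting the next attack whenever the chain montage is not playing and cycling through four steps.
; The combo count selects the montage section by name.
; After release, once the attack ends, the matching recovery section plays and the count resets.
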(event `InputAxis|MousePitch`
  (params (AxisValue :type "Float (single-precision)"))
  (`self.AddControllerPitchInput` AxisValue))

(event `InputAction|Jump`
  (params (Key :type "Key Structure"))
  (:`Pressed`
    (`self.Jump`)))

(event `InputAxis|MouseYaw`
  (params (AxisValue :type "Float (single-precision)"))
  (`self.AddControllerYawInput` AxisValue))

(event `InputAction|LeftMouseButton`
  (params (Key :type "Key Structure"))
  (:`Pressed`
    (set `self.LeftMouseDown?` true))
  (:`Released`
    (set `self.LeftMouseDown?` false)))

(event `self.ReceiveTick`
  (params (DeltaSeconds :type "Float (single-precision)"))
  (bind _returnvalue (`AnimInstance.Montage_IsPlaying` (`SkeletalMeshComponent.GetAnimInstance` (`self.Mesh`)) "/Game/MyShishleStuff/Serath_AttackChain.Serath_AttackChain"))
  (if (`self.LeftMouseDown?`)
    (if (not _returnvalue)
      (if (<= (`self.ComboCount`) 3)
        (bind _result (`/Engine/EditorBlueprintResources/StandardMacros.IncrementInt` (`self.ComboCount`))
          (:`  `
            (set `self.ComboCount` _result)))
        (else
          (set `self.ComboCount` 1)))
      (`self.PlayAnimMontage` "/Game/MyShishleStuff/Serath_AttackChain.Serath_AttackChain" 1.0 (`KismetStringLibrary.Conv_StringToName` (`KismetStringLibrary.Conv_IntToString` (`self.ComboCount`)))))
    (elif (and (> (`self.ComboCount`) 0) (not _returnvalue))
      (`self.PlayAnimMontage` "/Game/MyShishleStuff/Serath_AttackRecovery.Serath_AttackRecovery" 1.0 (`KismetStringLibrary.Conv_StringToName` (`KismetStringLibrary.Conv_IntToString` (`self.ComboCount`))))
      (set `self.ComboCount` 0))))

(fn `UserConstructionScript`)